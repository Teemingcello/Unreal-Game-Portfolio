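; Whiteboard Blueprint that can be drawn on at runtime through a render target.
; BeginPlay creates a render target, a brush material instance (M_WhiteBoardMaker) and a mesh material (M_WhiteBoard) that displays the target.
; DrawOnWhiteBoard feeds a 2D location into the brush material and draws it to the render target.
; DrawSize sets the brush's size parameter for subsequent draws.
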(event Custom|DrawOnWhiteBoard
  (params (LocationToDraw :type Vector%202D%20Structure))
  (Rendering|Material|SetVectorParameterValue (Variables|Default|GetWhiteBoardMaker) "DrawLocation" (Math|Conversions|ToLinearColor(Vector) (Math|Conversions|ToVector(Vector2D) LocationToDraw 0.1)) :!class /Script/Engine.MaterialInstanceDynamic)
  (Rendering|DrawMaterialtoRenderTarget (Variables|Default|GetRT%20Texture) (Variables|Default|GetWhiteBoardMaker)))

(event Custom|DrawSize
  (params (DrawSize :type Float%20%28double-precision%29))
  (Rendering|Material|SetScalarParameterValue (Variables|Default|GetWhiteBoardMaker) "DrawSize" DrawSize :!class /Script/Engine.MaterialInstanceDynamic))

(event EventBeginPlay
  (bind _returnvalue (Rendering|Material|CreateDynamicMaterialInstance "/Game/RenderTarget/M_WhiteBoardMaker.M_WhiteBoardMaker" "None" "None" :!class /Script/Engine.KismetMaterialLibrary))
  (Variables|Default|SetWhiteBoardMaker _returnvalue)
  (bind _returnvalue_2 (Rendering|CreateRenderTarget2D 512 512 "RTF_RGBA16f" "(R=0.000000,G=0.000000,B=0.000000,A=1.000000)" true))
  (Variables|Default|SetRT%20Texture _returnvalue_2)
  (bind _returnvalue_3 (Rendering|Material|CreateDynamicMaterialInstance (Variables|Default|GetStaticMesh) 0 "/Game/RenderTarget/M_WhiteBoard.M_WhiteBoard" "None" :!class /Script/Engine.PrimitiveComponent))
  (Rendering|Material|SetTextureParameterValue _returnvalue_3 "RT_Texture" (Variables|Default|GetRT%20Texture)))

(fn ConstructionScript)