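; Paintable mesh canvas actor that records hits as brush stamps in render targets, with separate paint and erase events.
; On BeginPlay it creates base and deform render targets, seeds the base with a splat texture, and binds both to the mesh's dynamic material.
; Paint hits draw a randomly sized, rotated color brush into the base target at the hit UV.
; Erase hits draw a smaller brush into the deform target.
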(event Custom|Apply%20Hit%20Erase
  (params (UVHit :type Vector%202D%20Structure) (HitNormal :type Vector))
  (Development|PrintString (Utilities|String|ToString(Vector2d) UVHit))
  (Development|PrintString (Utilities|String|ToString(Integer) HitNormal))
  (Utilities|FlowControl|Sequence
    (:then_0
      (bind (_canvas _size _context) (Rendering|BeginDrawCanvastoRenderTarget (Variables|Default|GetCRT_Deform)))
      (Canvas|DrawMaterial :self _canvas :RenderMaterial (Variables|Default|GetDeformMaterial) :ScreenPosition (.Screen%20Position (CallFunction|SetCanvasMaterialScaleandPosition _size UVHit (Math|Random|RandomFloatinRange 0.03 0.05))) :ScreenSize (.Screen%20Size (CallFunction|SetCanvasMaterialScaleandPosition _size UVHit (Math|Random|RandomFloatinRange 0.03 0.05))) :CoordinateSize "(X=1.000000,Y=1.000000)" :PivotPoint "(X=0.500000,Y=0.500000)")
      (Rendering|EndDrawCanvastoRenderTarget _context))))

(event Custom|Apply%20Hit%20Painting
  (params (UVHit :type Vector%202D%20Structure) (HitNormal :type Vector))
  (Development|PrintString (Utilities|String|ToString(Vector2d) UVHit))
  (Development|PrintString (Utilities|String|ToString(Integer) HitNormal))
  (Utilities|FlowControl|Sequence
    (:then_1
      (bind (_canvas _size _context) (Rendering|BeginDrawCanvastoRenderTarget (Variables|Default|GetCRT_Base)))
      (Canvas|DrawMaterial :self _canvas :RenderMaterial (Variables|Default|GetBaseColorMaterial) :ScreenPosition (.Screen%20Position (CallFunction|SetCanvasMaterialScaleandPosition _size UVHit (Math|Random|RandomFloatinRange 0.25 0.3))) :ScreenSize (.Screen%20Size (CallFunction|SetCanvasMaterialScaleandPosition _size UVHit (Math|Random|RandomFloatinRange 0.25 0.3))) :CoordinateSize "(X=1.000000,Y=1.000000)" :Rotation (Math|Random|RandomFloatinRange 0.0 3.6e+02) :PivotPoint "(X=0.500000,Y=0.500000)")
      (Rendering|EndDrawCanvastoRenderTarget _context))))

(event EventBeginPlay
  (CallFunction|InitializeCanvasRenderTarget))

(fn ConstructionScript)

(fn InitializeCanvasRenderTarget
  (Utilities|FlowControl|Sequence
    (:then_0
      (bind _returnvalue (Rendering|Material|CreateDynamicMaterialInstance (Variables|Debug|GetStaticMeshComponent) 0 "/Game/RenderTarget/M_NewMaterial.M_NewMaterial" "None" :!class /Script/Engine.PrimitiveComponent))
      (Variables|Default|SetCanvasMaterial _returnvalue))
    (:then_1
      (bind _returnvalue_2 (CanvasRenderTarget2D|CreateCanvasRenderTarget2D "/Script/Engine.CanvasRenderTarget2D" 1024 1024))
      (Variables|Default|SetCRT_Deform _returnvalue_2)
      (bind _returnvalue_3 (CanvasRenderTarget2D|CreateCanvasRenderTarget2D "/Script/Engine.CanvasRenderTarget2D" 1024 1024))
      (bind _output_get (Variables|Default|SetCRT_Base _returnvalue_3))
      (bind (_canvas _size _context) (Rendering|BeginDrawCanvastoRenderTarget _output_get))
      (Canvas|DrawTexture _canvas "/Game/VAT/PaintSplat_pos.PaintSplat_pos" "(X=0.000000,Y=0.000000)" _size "(X=0.000000,Y=0.000000)" "(X=1.000000,Y=1.000000)" "(R=1.000000,G=1.000000,B=1.000000,A=1.000000)" "BLEND_Translucent" 0.0 "(X=0.500000,Y=0.500000)")
      (Rendering|EndDrawCanvastoRenderTarget _context))
    (:then_2
      (bind _returnvalue_4 (Rendering|Material|CreateDynamicMaterialInstance "/Game/RenderTarget/M_DeformBrush.M_DeformBrush" "None" "None" :!class /Script/Engine.KismetMaterialLibrary))
      (Variables|Default|SetDeformMaterial _returnvalue_4))
    (:then_3
      (bind _returnvalue_5 (Rendering|Material|CreateDynamicMaterialInstance "/Game/RenderTarget/M_BaseColorBrush.M_BaseColorBrush" "None" "None" :!class /Script/Engine.KismetMaterialLibrary))
      (Variables|Default|SetBaseColorMaterial _returnvalue_5))
    (:then_4
      (Rendering|Material|SetTextureParameterValue (Variables|Default|GetCanvasMaterial) "DeformTexture" (Variables|Default|GetCRT_Deform))
      (Rendering|Material|SetTextureParameterValue (Variables|Default|GetCanvasMaterial) "BaseTexture" (Variables|Default|GetCRT_Base)))))