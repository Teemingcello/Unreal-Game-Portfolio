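; Bouncing projectile that erases paint from BP_Canvas actors it hits, destroying itself once it exceeds its bounce limit.
; On a canvas hit, a short complex line trace along its forward vector finds the collision UV.
; It passes that UV to the canvas's ApplyHitErase, with the normalized trace direction as HitNormal rather than the surface normal.
; Debug prints remain, and the physics impulse logic is disconnected.
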(event Collision|EventHit
  (params (MyComp :type Primitive%20Component%20Object%20Reference) (Other :type Actor%20Object%20Reference) (OtherComp :type Primitive%20Component%20Object%20Reference) (bSelfMoved :type Boolean) (HitLocation :type Vector :default "0, 0, 0") (HitNormal :type Vector :default "0, 0, 0") (NormalImpulse :type Vector :default "0, 0, 0") (Hit :type Hit%20Result%20Structure%20%28by%20ref%29))
  (bind _returnvalue (Transformation|GetActorLocation))
  (Math|Integer|IncrementInt (Variables|Default|GetBounce)
    (:%20%20
      (if (> (Variables|Default|GetBounce) 5)
        (Actor|DestroyActor) ; Then destroy this projectile
        (else
          ;[1 1 1] Canvas Hit
          (bind _asbp_canvas (Utilities|Casting|CastToBP_Canvas Other))
          (Development|PrintString (Utilities|GetDisplayName Other))
          (bind (_outhit _returnvalue_2) (Collision|LineTraceByChannel _returnvalue (+ _returnvalue (* (Math|Vector|GetForwardVector (Transformation|GetActorRotation)) 1e+02)) "TraceTypeQuery1" true 0 "None"))
          (if _returnvalue_2
            (Development|PrintString (Utilities|String|ToString(Boolean) (.ReturnValue (Class|GameplayStatics|FindCollisionUV _outhit))))
            (Default|ApplyHitErase _asbp_canvas (.UV (Class|GameplayStatics|FindCollisionUV _outhit)) (Math|Vector|Normalize (- (.TraceEnd (Collision|BreakHitResult _outhit)) (.TraceStart (Collision|BreakHitResult _outhit)))))))))))

(fn ConstructionScript)