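; Bouncing paintball projectile that splatters paint on hits and paints BP_Canvas actors, destroying itself after a bounce limit.
; Each hit spawns a splat emitter whose particle collisions place randomly rolled decals, using a dynamic material given a render target at BeginPlay.
; On canvas hits, a forward complex trace finds the collision UV and passes it to ApplyHitPainting.
; The physics impulse branch is disconnected and never runs.
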(event Custom|BallPaint_OnParticleCollide
  (params (EventName :type Name) (EmitterTime :type Float%20%28single-precision%29) (ParticleTime :type Integer) (Location :type Vector) (Velocity :type Vector) (Direction :type Vector) (Normal :type Vector) (BoneName :type Name) (PhysMat :type Physical%20Material%20Object%20Reference))
  (bind _returnvalue (Rendering|Decal|SpawnDecalatLocation (Variables|Default|GetDecalMaterial) "128.000000,128.000000,128.000000" Location (Math|Rotator|Lerp(Rotator) (Math|Rotator|MakeRotfromX (stale Collision|EventHit HitNormal)) (Class|KismetMathLibrary|MakeRotfromYZ (stale Collision|EventHit HitNormal) (stale Collision|EventHit HitNormal)) 2.0) 0.0))
  (Transformation|AddRelativeRotation _returnvalue (Math|Rotator|MakeRotator (Math|Random|RandomFloatinRange 0.0 3.6e+02) 0.0 0.0) false false))

(event EventBeginPlay
  (bind _returnvalue (Rendering|Material|CreateDynamicMaterialInstance "/Game/Projectile/BallPaint/M_SplatDecal.M_SplatDecal" "None" "None" :!class /Script/Engine.KismetMaterialLibrary))
  (bind _output_get (Variables|Default|SetDecalMaterial _returnvalue))
  (bind _returnvalue_2 (Rendering|CreateRenderTarget2D 512 512 "RTF_RGBA16f" "(R=0.000000,G=0.000000,B=0.000000,A=1.000000)" true))
  (bind _output_get_2 (Variables|Default|SetRT%20Texture _returnvalue_2))
  (Rendering|Material|SetTextureParameterValue _output_get "RT_Texture" _output_get_2))

(event Collision|EventHit
  (params (MyComp :type Primitive%20Component%20Object%20Reference) (Other :type Actor%20Object%20Reference) (OtherComp :type Primitive%20Component%20Object%20Reference) (bSelfMoved :type Boolean) (HitLocation :type Vector :default "0, 0, 0") (HitNormal :type Vector :default "0, 0, 0") (NormalImpulse :type Vector :default "0, 0, 0") (Hit :type Hit%20Result%20Structure%20%28by%20ref%29))
  (bind _returnvalue (Transformation|GetActorLocation))
  (Math|Integer|IncrementInt (Variables|Default|GetBounce)
    (:%20%20
      (if (> (Variables|Default|GetBounce) 5)
        (Actor|DestroyActor) ; Then destroy this projectile
        (else
          (bind _returnvalue_2 (Effects|SpawnEmitteratLocation "/Game/Projectile/BallPaint/FX_Paintsplat.FX_Paintsplat" (Transformation|GetActorLocation)))
          (EventDispatchers|BindEventtoOnParticleCollide _returnvalue_2 (delegate Custom|BallPaint_OnParticleCollide))
          ;[1 1 1] Canvas Hit
          (bind _asbp_canvas (Utilities|Casting|CastToBP_Canvas Other))
          (bind (_outhit _returnvalue_3) (Collision|LineTraceByChannel _returnvalue (+ _returnvalue (* (Math|Vector|GetForwardVector (Transformation|GetActorRotation)) 1e+02)) "TraceTypeQuery1" true 0 "None"))
          (if _returnvalue_3
            (Development|PrintString (Utilities|String|ToString(Boolean) (.ReturnValue (Class|GameplayStatics|FindCollisionUV _outhit))))
            (Default|ApplyHitPainting _asbp_canvas (.UV (Class|GameplayStatics|FindCollisionUV _outhit)) (Math|Vector|Normalize (- (.TraceEnd (Collision|BreakHitResult _outhit)) (.TraceStart (Collision|BreakHitResult _outhit)))))))))))

(fn ConstructionScript)