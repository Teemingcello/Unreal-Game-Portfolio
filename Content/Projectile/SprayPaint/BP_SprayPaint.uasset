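; BP_SprayPaint is a spray paint projectile actor for the paint rifle that applies erase hits to canvases.
; StartFiring activates the particle spray and binds its collision event plus the rifle's stop-auto-fire event.
; Each particle collision sphere-traces along the particle direction, finds the collision UV and passes it to BP_Canvas.ApplyHitErase with the trace direction as normal.
; StopFiring deactivates the spray and destroys the actor after a delay.
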(event Custom|Start%20Firing
  (params (Paint%20Rifle :type BP%20Spray%20Rifle%20Object%20Reference))
  ;[1 1 1] 자동 연사 시작
  (EventDispatchers|BindEventtoOnStopAutoFire Paint%20Rifle (EventDispatchers|CreateEvent :!event Custom|Stop%20Firing))
  (Components|Activation|Activate (Variables|Default|GetSprayPaint) false)
  (EventDispatchers|BindEventtoOnParticleCollide (Variables|Default|GetSprayPaint) (delegate Custom|SprayCollide)))

(event Custom|Stop%20Firing
  ;[1 1 1] 자동 연사 종료
  (Components|Activation|Deactivate (Variables|Default|GetSprayPaint))
  (Utilities|FlowControl|Delay 5.0)
  (Actor|DestroyActor))

(event Custom|SprayCollide
  (params (EventName :type Name) (EmitterTime :type Float%20%28single-precision%29) (ParticleTime :type Integer) (Location :type Vector) (Velocity :type Vector) (Direction :type Vector) (Normal :type Vector) (BoneName :type Name) (PhysMat :type Physical%20Material%20Object%20Reference))
  ;[1 1 1] Canvas Hit
  (bind (_outhit _returnvalue) (Collision|SphereTraceForObjects Location (+ Location (* Direction 5e+01)) 1e+01 (Utilities|Array|MakeArray "ObjectTypeQuery2" "ObjectTypeQuery1") false 0 "None"))
  (if _returnvalue
    (bind _asbp_canvas (Utilities|Casting|CastToBP_Canvas (.HitActor (Collision|BreakHitResult _outhit))))
    (Development|PrintString (Utilities|String|ToString(Boolean) (.ReturnValue (Class|GameplayStatics|FindCollisionUV _outhit))))
    (Default|ApplyHitErase _asbp_canvas (.UV (Class|GameplayStatics|FindCollisionUV _outhit)) (Math|Vector|Normalize (- (.TraceEnd (Collision|BreakHitResult _outhit)) (.TraceStart (Collision|BreakHitResult _outhit)))))))

(fn ConstructionScript)

(fn SprayDrawing)