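; Shotgun paint spray actor that emits a short particle burst and applies erase hits to BP_Canvas surfaces it strikes.
; BeginPlay binds the particle collision event and deactivates the emitter after a brief delay.
; Each collision sphere-traces along the particle direction, then passes the collision UV and normalized trace direction (as the normal) to ApplyHitErase, printing a debug value.
; ShotGunStartFiring destroys the actor after a delay.
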(event Custom|Shot%20Gun%20Start%20Firing
  (Utilities|FlowControl|Delay 5.0)
  (Actor|DestroyActor))

(event Custom|SprayShot_Collide
  (params (EventName :type Name) (EmitterTime :type Float%20%28single-precision%29) (ParticleTime :type Integer) (Location :type Vector) (Velocity :type Vector) (Direction :type Vector) (Normal :type Vector) (BoneName :type Name) (PhysMat :type Physical%20Material%20Object%20Reference))
  ;[1 1 1] Canvas Hit
  (bind (_outhit _returnvalue) (Collision|SphereTraceForObjects Location (+ Location (* Direction 1e+02)) 25.0 (Utilities|Array|MakeArray "ObjectTypeQuery2") false 0 "None"))
  (if _returnvalue
    (bind _asbp_canvas (Utilities|Casting|CastToBP_Canvas (.HitActor (Collision|BreakHitResult _outhit))))
    (Development|PrintString (Utilities|String|ToString(Boolean) (.ReturnValue (Class|GameplayStatics|FindCollisionUV _outhit))))
    (Default|ApplyHitErase _asbp_canvas (.UV (Class|GameplayStatics|FindCollisionUV _outhit)) (Math|Vector|Normalize (- (.TraceEnd (Collision|BreakHitResult _outhit)) (.TraceStart (Collision|BreakHitResult _outhit)))))))

(event EventBeginPlay
  (EventDispatchers|BindEventtoOnParticleCollide (Variables|Default|GetShotGunPaint) (delegate Custom|SprayShot_Collide))
  (Utilities|FlowControl|Delay 0.2)
  (Components|Activation|Deactivate (Variables|Default|GetShotGunPaint)))

(fn ConstructionScript)