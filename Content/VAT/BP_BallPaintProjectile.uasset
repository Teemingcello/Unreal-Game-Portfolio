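; BP_BallPaintProjectile is a projectile that leaves a paint splat decal on whatever it hits.
; BeginPlay creates a dynamic M_SplatDecal material and feeds it a new render target, which nothing here draws into.
; On hit it spawns a splat emitter, stops, destroys itself and attaches a randomly sized and rolled decal aligned to the hit normal.
; A physics impulse branch exists but is disconnected.
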(event EventBeginPlay
  (bind _returnvalue (Rendering|Material|CreateDynamicMaterialInstance "/Game/VAT/M_SplatDecal.M_SplatDecal" "None" "None" :!class /Script/Engine.KismetMaterialLibrary))
  (bind _output_get (Variables|Default|SetDecalMaterial _returnvalue))
  (bind _returnvalue_2 (Rendering|CreateRenderTarget2D 512 512 "RTF_RGBA16f" "(R=0.000000,G=0.000000,B=0.000000,A=1.000000)" true))
  (bind _output_get_2 (Variables|Default|SetRT%20Texture _returnvalue_2))
  (Rendering|Material|SetTextureParameterValue _output_get "RT_Texture" _output_get_2))

(event Collision|EventHit
  (params (MyComp :type Primitive%20Component%20Object%20Reference) (Other :type Actor%20Object%20Reference) (OtherComp :type Primitive%20Component%20Object%20Reference) (bSelfMoved :type Boolean) (HitLocation :type Vector :default "0, 0, 0") (HitNormal :type Vector :default "0, 0, 0") (NormalImpulse :type Vector :default "0, 0, 0") (Hit :type Hit%20Result%20Structure%20%28by%20ref%29))
  (bind _returnvalue (Transformation|GetActorLocation))
  (Effects|SpawnEmitteratLocation "/Game/VAT/FX_Paintsplat.FX_Paintsplat" _returnvalue)
  (Components|Movement|StopMovementImmediately (Variables|MyProjectile|GetProjectile))
  (Actor|DestroyActor) ; Then destroy this projectile
  (bind _returnvalue_2 (Class|GameplayStatics|SpawnDecalAttached (Variables|Default|GetDecalMaterial) (Math|Vector|MakeVector (Math|Random|RandomFloatinRange -3e+01 -7e+01) (Math|Random|RandomFloatinRange 1.1e+02 1.5e+02) (Math|Random|RandomFloatinRange 1.1e+02 1.5e+02)) OtherComp "None" _returnvalue (Math|Rotator|MakeRotfromX HitNormal) "KeepWorldPosition" 0.0))
  (bind _output_get (Variables|Default|SetPaintDecal _returnvalue_2))
  (Transformation|AddRelativeRotation _output_get (Math|Rotator|MakeRotator (Math|Random|RandomFloatinRange 0.0 3.6e+02) 0.0 0.0) false false))

(fn ConstructionScript)