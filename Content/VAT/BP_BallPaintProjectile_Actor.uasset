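; Paintball projectile actor that bursts into a splat effect on impact and leaves a paint mark through a spawned BP_Chromatic.
; BeginPlay creates a render target and feeds it into a dynamic splat decal material, while DrawOnWhiteBoard and DrawSize events allow painting into it.
; On hit it stops, destroys itself and passes that material to BP_Chromatic with a randomized size.
; Physics impulse, direct decal and random rotation logic are left disconnected.
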(event Custom|DrawOnWhiteBoard
  (params (LocationToDraw :type Vector%202D%20Structure))
  (Rendering|Material|SetVectorParameterValue (Variables|Default|GetWhiteBoardMaker) "DrawLocation" (Math|Conversions|ToLinearColor(Vector) (Math|Conversions|ToVector(Vector2D) LocationToDraw 0.1)) :!class /Script/Engine.MaterialInstanceDynamic)
  (Rendering|DrawMaterialtoRenderTarget (Variables|Default|GetRT%20Texture) (Variables|Default|GetWhiteBoardMaker)))

(event Custom|DrawSize
  (params (DrawSize :type Float%20%28double-precision%29))
  (Rendering|Material|SetScalarParameterValue (Variables|Default|GetWhiteBoardMaker) "DrawSize" DrawSize :!class /Script/Engine.MaterialInstanceDynamic))

(event EventBeginPlay
  (bind _returnvalue (Rendering|Material|CreateDynamicMaterialInstance "/Game/VAT/M_SplatDecal.M_SplatDecal" "None" "None" :!class /Script/Engine.KismetMaterialLibrary))
  (Variables|Default|SetDecalMaterial _returnvalue)
  (bind _returnvalue_2 (Rendering|Material|CreateDynamicMaterialInstance "/Game/RenderTarget/M_WhiteBoardMaker.M_WhiteBoardMaker" "None" "None" :!class /Script/Engine.KismetMaterialLibrary))
  (Variables|Default|SetWhiteBoardMaker _returnvalue_2)
  (bind _returnvalue_3 (Rendering|CreateRenderTarget2D 512 512 "RTF_RGBA16f" "(R=0.000000,G=0.000000,B=0.000000,A=1.000000)" true))
  (bind _output_get (Variables|Default|SetRT%20Texture _returnvalue_3))
  (Rendering|Material|SetTextureParameterValue (Variables|Default|GetDecalMaterial) "RT_Texture" _output_get))

(event Collision|EventHit
  (params (MyComp :type Primitive%20Component%20Object%20Reference) (Other :type Actor%20Object%20Reference) (OtherComp :type Primitive%20Component%20Object%20Reference) (bSelfMoved :type Boolean) (HitLocation :type Vector :default "0, 0, 0") (HitNormal :type Vector :default "0, 0, 0") (NormalImpulse :type Vector :default "0, 0, 0") (Hit :type Hit%20Result%20Structure%20%28by%20ref%29))
  (bind _returnvalue (Transformation|GetActorLocation))
  (Effects|SpawnEmitteratLocation "/Game/VAT/FX_Paintsplat.FX_Paintsplat" _returnvalue)
  (Components|Movement|StopMovementImmediately (Variables|MyProjectile|GetProjectile))
  (Actor|DestroyActor) ; Then destroy this projectile
  (bind _returnvalue_2 (Game|SpawnActorfromClass "/Game/RenderTarget/BP_Chromatic.BP_Chromatic_C" (Transformation|GetActorTransform) "Undefined" 0 0))
  (Default|CreateChromatic _returnvalue_2 (Variables|Default|GetDecalMaterial) (Math|Vector|MakeVector (Math|Random|RandomFloatinRange -3e+01 -7e+01) (Math|Random|RandomFloatinRange 1.1e+02 1.5e+02) (Math|Random|RandomFloatinRange 1.1e+02 1.5e+02)) _returnvalue "0, 0, 0"))

(fn ConstructionScript)